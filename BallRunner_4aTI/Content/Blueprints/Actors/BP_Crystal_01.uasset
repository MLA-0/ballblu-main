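; BP_Crystal_01 is a crystal actor that plays a collect-style vanish animation when something overlaps its sphere.
; The overlap caches location, scale and light intensity, then starts the Crystal timeline.
; Each timeline update lerps the crystal toward player pawn 0's current position while shrinking it to zero and fading its point light.
; The actor destroys itself when the timeline finishes, with no overlap filtering or reward logic.
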(event OnComponentBeginOverlap(Sphere)
  (params (OverlappedComponent :type Primitive%20Component%20Object%20Reference) (OtherActor :type Actor%20Object%20Reference) (OtherComp :type Primitive%20Component%20Object%20Reference) (OtherBodyIndex :type Integer) (bFromSweep :type Boolean) (SweepResult :type Hit%20Result%20Structure%20%28by%20ref%29))
  (CallFunction|NewFunction3)
  (bind (_direction _crystallocation _2 _swiatlo) (Timeline|Crystal Play)
    (:Update
      (CallFunction|NewFunction0 _crystallocation)
      (CallFunction|NewFunction1 _2)
      (CallFunction|NewFunction2 _swiatlo))
    (:Finished
      (Actor|DestroyActor))))

(fn ConstructionScript)

(fn NewFunction0
  (params (Alpha :type Float%20%28single-precision%29))
  (Transformation|SetActorLocation (Math|Vector|Lerp(Vector) (Variables|Default|Getcrystal_location) (Transformation|GetActorLocation (Game|Player|GetPlayerPawn 0)) Alpha) false false))

(fn NewFunction1
  (params (Alpha :type Float%20%28single-precision%29))
  (Transformation|SetActorScale3D (Math|Vector|Lerp(Vector) (Variables|Default|Getcrystal_scale) "0, 0, 0" Alpha)))

(fn NewFunction2
  (params (Alpha :type Float%20%28single-precision%29))
  (Rendering|Components|Light|SetIntensity (Variables|Default|GetPointLight) (Math|Float|Lerp (Variables|Default|Getcrystal_light) 0.0 Alpha)))

(fn NewFunction3
  (Variables|Default|Setcrystal_location (Transformation|GetActorLocation))
  (Variables|Default|Setcrystal_scale (Transformation|GetActorScale3D))
  (Variables|Default|Setcrystal_light (Variables|/Script/Engine.LightComponentBase|GetIntensity (Variables|Default|GetPointLight))))